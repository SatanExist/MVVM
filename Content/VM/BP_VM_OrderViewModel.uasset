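; BP_VM_OrderViewModel is a view model for an ordering screen that prepares child view models for the available drinks and addons.
; CreateVMObjects constructs a BP_VM_OrderItem for each available drink and a BP_VM_OrderAddon for each available addon, copying the entry into its name field.
; Each new object gets a field-change broadcast and is stored in InitializedDrinks or InitializedAddons.
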(fn CreateVMObjects
  ;[0.15 0.0728 0.1424 0.5] Create VM_OrderAddons
  (for _array_element (Variables|Default|GetAvailableDrinks)
    (bind _returnvalue (Game|ConstructObjectfromClass "/Game/VM/BP_VM_OrderItem.BP_VM_OrderItem_C"))
    (Variables|/Script/MVVM3.VM_OrderItem|SetItemName _returnvalue _array_element)
    (FieldNotification|BroadcastFieldValueChanged _returnvalue "(FieldName=\"ItemName\")")
    (Utilities|Array|Add (Variables|Default|GetInitializedDrinks) _returnvalue))
  ;[0.07006 0.15 0 0.46] Create VM_OrderItems
  (for _array_element_2 (Variables|Default|GetAvailableAddons)
    (bind _returnvalue_2 (Game|ConstructObjectfromClass "/Game/VM/BP_VM_OrderAddon.BP_VM_OrderAddon_C"))
    (Variables|/Script/MVVM3.VM_OrderAddon|SetAddonName _returnvalue_2 _array_element_2)
    (FieldNotification|BroadcastFieldValueChanged _returnvalue_2 "(FieldName=\"AddonName\")")
    (Utilities|Array|Add (Variables|Default|GetInitializedAddons) _returnvalue_2)))